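; Heart pickup actor that heals the Player by one life point on overlap and destroys itself.
; BeginPlay caches the spawn location and offsets MaxHeight from it, then Tick bobs the heart vertically using a sine of accumulated time as the Lerp alpha, swinging above and below the origin.
; The SetNotPersistent event makes the heart temporary by destroying it after DespawnTimer.
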(event `SetNotPersistent`
  (`KismetSystemLibrary.Delay` (`self.despawnTimer`))
  (`self.K2_DestroyActor`))

(event `self.ReceiveBeginPlay`
  (`self.setDefaultValues`))

(event `self.ReceiveActorBeginOverlap`
  (params (OtherActor :type "Actor Object Reference"))
  (bind _asplayer (cast `/Game/Blueprints/Player` OtherActor))
  (`self.K2_DestroyActor`)
  (`/Game/Components/LifeComponent.heal` (`/Game/Blueprints/Player.playerLife` _asplayer) 1))

(event `self.ReceiveTick`
  (params (DeltaSeconds :type "Float (single-precision)"))
  ;[1 1 1] Tick
  (set `self.timeCounter` (+ DeltaSeconds (`self.timeCounter`)))
  (`self.move`))

(fn `move`
  (bind (_origin_x _origin_y _origin_z) (`KismetMathLibrary.BreakVector` (`self.origin`)))
  (`self.K2_SetActorLocationAndRotation` (`KismetMathLibrary.MakeVector` _origin_x _origin_y (`KismetMathLibrary.Lerp` _origin_z (`self.maxHeight`) (`KismetMathLibrary.Sin` (`self.timeCounter`)))) (`self.initialRotation`)))

(fn `setDefaultValues`
  (bind (_returnvalue_x _returnvalue_y _returnvalue_z) (`KismetMathLibrary.BreakVector` (`self.K2_GetActorLocation`)))
  (set `self.maxHeight` (+ (`self.maxHeight`) _returnvalue_z))
  (set `self.origin` (`KismetMathLibrary.MakeVector` _returnvalue_x _returnvalue_y _returnvalue_z)))

(fn `UserConstructionScript`)